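; MouseController makes the character's DominoTile follow the mouse cursor through the 3D world.
; Each Tick, it reads the tile from DominoGameCharacter and line traces on Visibility from just ahead of the character toward a distant point along the deprojected cursor ray.
; The trace ignores the tile, leaves debug drawing on, and moves the tile to any hit location without sweeping.
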(event EventBeginPlay)

(event EventTick
  (params (DeltaSeconds :type Float%20%28single-precision%29))
  (bind (_worldlocation _worlddirection) (Game|Player|ConvertMouseLocationToWorldSpace))
  (bind _returnvalue (Game|GetPlayerCharacter 0))
  ;[1 1 1] Cast to my character blueprint for tool variable
  (bind _asdomino_game_character (Utilities|Casting|CastToDominoGameCharacter (Game|GetPlayerCharacter 0)))
  ;[1 1 1] Cast from player to mouse position in 3D Space
  (bind (_outhit _returnvalue_2) (Collision|LineTraceByChannel (+ (Transformation|GetActorLocation _returnvalue) (Transformation|GetActorForwardVector _returnvalue)) (+ _worldlocation (* _worlddirection 2e+03)) "TraceTypeQuery1" false (Utilities|Array|MakeArray (Variables|/Game/Blueprints/DominoGameCharacter.DominoGameCharacter_C|GetDominoTile _asdomino_game_character)) "ForDuration"))
  (if _returnvalue_2
    ;[1 1 1] If cast hit something then place the object at that location
    (Transformation|SetActorLocation (Variables|/Game/Blueprints/DominoGameCharacter.DominoGameCharacter_C|GetDominoTile _asdomino_game_character) (.Location (Collision|BreakHitResult _outhit)) false false)))

(fn ConstructionScript)