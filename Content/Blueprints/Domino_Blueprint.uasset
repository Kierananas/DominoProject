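; Draggable domino actor that shows pips and text for its head and tail values and follows the cursor while held, turning doubles 90 degrees.
; Release places it if valid or an initial placement, otherwise flags it spawned.
; Head overlaps inside the play area compare both dominoes; only tail-to-tail matches validate, rotating and placing the cursor-hit domino without collision.
; Tail-overlap logic is disconnected, and debug prints abound.
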(event OnComponentBeginOverlap(Compare_Tail)
  (params (OverlappedComponent :type Primitive%20Component%20Object%20Reference) (OtherActor :type Actor%20Object%20Reference) (OtherComp :type Primitive%20Component%20Object%20Reference) (OtherBodyIndex :type Integer) (bFromSweep :type Boolean) (SweepResult :type Hit%20Result%20Structure%20%28by%20ref%29)))

(event OnComponentBeginOverlap(Compare_Head)
  (params (OverlappedComponent :type Primitive%20Component%20Object%20Reference) (OtherActor :type Actor%20Object%20Reference) (OtherComp :type Primitive%20Component%20Object%20Reference) (OtherBodyIndex :type Integer) (bFromSweep :type Boolean) (SweepResult :type Hit%20Result%20Structure%20%28by%20ref%29))
  (bind _staticmeshcomponent (Variables|Debug|GetStaticMeshComponent))
  (switch Utilities|FlowControl|Switch|SwitchonDominoState (Variables|Default|GetDominoState)
    (:NewEnumerator1
      (bind _inarea (CallFunction|CheckPlayArea))
      (if _inarea
        ;[1 1 1] Reads Values from Right to Left
        (bind (_heads _tails) (CallFunction|CompareHeadMK2)) ; Get Values of Right Domino
        (bind _asdomino_blueprint (Utilities|Casting|CastToDomino_Blueprint OtherActor))
        (bind (_heads_2 _tails_2) (CallFunction|CompareHeadMK2 _asdomino_blueprint)) ; Get Values of Left Domino
        (bind (_head_equal_head _tail_equal_tail _head_equal_tail _tail_equal_head) (CallFunction|ComValue _heads _tails _heads_2 _tails_2 (Utilities|String|Append "Head" "Comparison")))
        (CallFunction|ReactFunction _head_equal_head _tail_equal_tail _head_equal_tail _tail_equal_head)
        (CallFunction|NewFunction0 (Transformation|GetWorldLocation _staticmeshcomponent) (Transformation|GetWorldLocation (Variables|/Script/Engine.Actor|GetRootComponent _asdomino_blueprint)) (Transformation|GetWorldScale _staticmeshcomponent) (Transformation|GetWorldScale (Variables|/Script/Engine.Actor|GetRootComponent _asdomino_blueprint)))
        (else
          (Development|PrintString "Out of Play Area"))))))

(event Collision|EventActorBeginOverlap
  (params (OtherActor :type Actor%20Object%20Reference)))

(event EventBeginPlay
  (CallFunction|InitData)
  (Physics|SetSimulatePhysics (Variables|Debug|GetStaticMeshComponent) true))

(event MouseInput|EventActorBeginCursorOver
  (Variables|/Script/Engine.PlayerController|SetCurrentMouseCursor (Game|GetPlayerController 0) "Hand"))

(event EventActorOnReleased
  (params (ButtonReleased :type Key%20Structure))
  (Variables|Default|SetDominoState "NewEnumerator2")
  (if (Variables|Default|GetIsValid)
    (Variables|Default|SetPlaced true :!label _label)
    (Development|PrintString "placed")
    (Variables|Default|SetInHand false)
    (elif (Variables|Default|GetIntialPlace)
      (goto _label)
      (else
        (Variables|Default|SetSpawned true)
        (Development|PrintString "Spawned")
        (Variables|Default|SetInHand false)))))

(event EventActorOnInputTouchBegin
  (params (FingerIndex :type ETouchIndex%20Enum :default "Touch1"))
  (Variables|Default|SetDominoState "NewEnumerator1")
  (Variables|Default|SetInHand true)
  (Development|PrintString "holding"))

(event EventActorOnInputTouchEnd
  (params (FingerIndex :type ETouchIndex%20Enum :default "Touch1"))
  (Variables|Default|SetDominoState "NewEnumerator2")
  (if (Variables|Default|GetIsValid)
    (Variables|Default|SetPlaced true :!label _label)
    (Development|PrintString "placed")
    (Variables|Default|SetInHand false)
    (elif (Variables|Default|GetIntialPlace)
      (goto _label)
      (else
        (Variables|Default|SetSpawned true)
        (Development|PrintString "Spawned")
        (Variables|Default|SetInHand false)))))

(event MouseInput|EventActorEndCursorOver
  (Variables|/Script/Engine.PlayerController|SetCurrentMouseCursor (Game|GetPlayerController 0) "Crosshairs"))

(event EventTick
  (params (DeltaSeconds :type Float%20%28single-precision%29))
  (bind _returnvalue (Game|GetPlayerController 0))
  (bind _hitresult (Game|Player|GetHitResultUnderCursorbyChannel _returnvalue "TraceTypeQuery1" true))
  (bind (_bblockinghit _binitialoverlap _time _distance _location _impactpoint _normal _impactnormal _physmat _hitactor) (Collision|BreakHitResult _hitresult))
  (bind (_x _y) (Math|Vector|BreakVector _location))
  ;[1 1 1] Domino Movement system MK 2 - Made in the Domino_Blueprint
  (switch Utilities|FlowControl|Switch|SwitchonDominoState (Variables|Default|GetDominoState)
    (:NewEnumerator1
      (if (== (Variables|Default|Gethead_value) (Variables|Default|Gettail_value))
        (Variables|Default|SetDomino%20Rotation "0,90.000000, 0")
        (else
          (Variables|Default|SetDomino%20Rotation "0, 0, 0")))
      (if (not (Variables|Default|GetPlaced))
        (Variables|Default|SetCurrentDomino _hitactor)
        (Transformation|SetActorLocation (Math|Vector|MakeVector _x _y (.Z (Math|Vector|BreakVector (Transformation|GetActorLocation)))) false true)
        (Transformation|SetActorRotation (Variables|Default|GetDomino%20Rotation))))))

(event MouseInput|EventActorOnClicked
  (params (ButtonPressed :type Key%20Structure))
  (Variables|Default|SetDominoState "NewEnumerator1")
  (Variables|Default|SetInHand true)
  (Development|PrintString "holding"))

(fn ConstructionScript
  (CallFunction|InitData))

(fn InitData
  (bind _tail_value (Variables|Default|Gettail_value))
  (bind _head_value (Variables|Default|Gethead_value))
  (CallFunction|HeadPips _head_value)
  (Rendering|Components|TextRender|SetText (Variables|Default|GetHead) (Utilities|Text|ToText(Integer) _head_value))
  (CallFunction|TailPips _tail_value)
  (Rendering|Components|TextRender|SetText (Variables|Default|GetTail) (Utilities|Text|ToText(Integer) _tail_value)))

(fn OnRepHeadValue)

(fn CompareValue)

(fn CompareTail
  (Utilities|FlowControl|Sequence
    (:then_0
      (Development|PrintString (Utilities|String|ToString(Integer) 0)))
    (:then_1
      (Development|PrintString (Utilities|String|ToString(Integer) 0)))
    (:then_2
      (Development|PrintString (Utilities|String|ToString(Integer) (Variables|Default|Gethead_value))))
    (:then_3
      (Development|PrintString (Utilities|String|ToString(Integer) (Variables|Default|Gettail_value))))))

(fn CompareHead
  (Utilities|FlowControl|Sequence
    (:then_0
      (Development|PrintString (Utilities|String|ToString(Integer) 0)))
    (:then_1
      (Development|PrintString (Utilities|String|ToString(Integer) 0)))
    (:then_2
      (Development|PrintString (Utilities|String|ToString(Integer) (Variables|Default|Gethead_value))))
    (:then_3
      (Development|PrintString (Utilities|String|ToString(Integer) (Variables|Default|Gettail_value))))))

(fn CompareTailMK2
  (bind _head_value (Variables|Default|Gethead_value))
  (bind _tail_value (Variables|Default|Gettail_value))
  (Utilities|FlowControl|Sequence
    (:then_0
      (Development|PrintString (Utilities|String|ToString(Integer) _head_value) true true "(R=1.000000,G=0.052905,B=0.000000,A=1.000000)" 3.0)
      (bind _output_get (Variables|Default|SetLeft_Head _head_value)))
    (:then_1
      (Development|PrintString (Utilities|String|ToString(Integer) _tail_value) true true "(R=1.000000,G=0.556244,B=0.000000,A=1.000000)" 3.0)
      (bind _output_get_2 (Variables|Default|SetLeft_Tail _tail_value)))
    (:then_2
      (return _output_get _output_get_2))))

(fn CompareHeadMK2
  (bind _head_value (Variables|Default|Gethead_value))
  (bind _tail_value (Variables|Default|Gettail_value))
  (Utilities|FlowControl|Sequence
    (:then_0
      (Development|PrintString (Utilities|String|ToString(Integer) _head_value) true true "(R=0.000000,G=1.000000,B=0.324472,A=1.000000)")
      (bind _output_get (Variables|Default|SetRight_Head _head_value)))
    (:then_1
      (Development|PrintString (Utilities|String|ToString(Integer) _tail_value) true true "(R=0.000000,G=0.705307,B=1.000000,A=1.000000)")
      (bind _output_get_2 (Variables|Default|SetRigth_Tail _tail_value)))
    (:then_2
      (return _output_get _output_get_2))))

(fn HeadPips
  (params (HeadValue :type Integer))
  (bind _pip_two_h (Variables|Default|GetPip_Two_H))
  (bind _pip_six_h (Variables|Default|GetPip_Six_H))
  (bind _pip_one_h (Variables|Default|GetPip_One_H))
  (switch Utilities|FlowControl|Switch|SwitchonHeadPips (Utilities|Enum|ByteToEnumHeadPips (Math|Conversions|ToByte(Integer) HeadValue))
    (:NewEnumerator0
      (Rendering|SetVisibility _pip_one_h false false))
    (:NewEnumerator1
      (Rendering|SetVisibility _pip_one_h true false)
      (Rendering|SetVisibility _pip_two_h false false))
    (:NewEnumerator2
      (Rendering|SetVisibility _pip_two_h true false)
      (Rendering|SetVisibility _pip_one_h false false))
    (:NewEnumerator3
      (Rendering|SetVisibility _pip_one_h true false)
      (Rendering|SetVisibility (Variables|Default|GetPip_Four_H) false false))
    (:NewEnumerator4
      (Rendering|SetVisibility _pip_two_h true false)
      (Rendering|SetVisibility _pip_one_h false false))
    (:NewEnumerator5
      (Rendering|SetVisibility (Variables|Default|GetPip_Five_H) true false)
      (Rendering|SetVisibility _pip_six_h false false))
    (:NewEnumerator6
      (Rendering|SetVisibility _pip_six_h true true)
      (Rendering|SetVisibility _pip_one_h false false))))

(fn TailPips
  (params (TailValue :type Integer))
  (bind _pip_one_t (Variables|Default|GetPip_One_T))
  (bind _pip_two_t (Variables|Default|GetPip_Two_T))
  (switch Utilities|FlowControl|Switch|SwitchonHeadPips (Utilities|Enum|ByteToEnumHeadPips (Math|Conversions|ToByte(Integer) TailValue))
    (:NewEnumerator0
      (Rendering|SetVisibility _pip_one_t false false))
    (:NewEnumerator1
      (Rendering|SetVisibility _pip_one_t true false)
      (Rendering|SetVisibility _pip_two_t false false))
    (:NewEnumerator2
      (Rendering|SetVisibility _pip_two_t true false)
      (Rendering|SetVisibility _pip_one_t false false))
    (:NewEnumerator3
      (Rendering|SetVisibility _pip_two_t true false)
      (Rendering|SetVisibility (Variables|Default|GetPip_Four_T) false false))
    (:NewEnumerator4
      (Rendering|SetVisibility _pip_two_t true false)
      (Rendering|SetVisibility _pip_one_t false false))
    (:NewEnumerator5
      (Rendering|SetVisibility (Variables|Default|GetPip_Five_T) true false)
      (Rendering|SetVisibility (Variables|Default|GetPip_Six_T) false false))
    (:NewEnumerator6
      (Rendering|SetVisibility (Variables|Default|GetPip_Six1_T) true true)
      (Rendering|SetVisibility _pip_one_t false false))))

(fn CompareVal
  (params (Tail_Self_Head :type Integer%20%28by%20ref%29) (Tail_Self_Tail :type Integer%20%28by%20ref%29) (Tail_Cast_Head :type Integer%20%28by%20ref%29) (Tail_Cast_Tail :type Integer%20%28by%20ref%29) (Tail :type String%20%28by%20ref%29) (Head_Self_Head :type Integer%20%28by%20ref%29) (Head_Self_Tail :type Integer%20%28by%20ref%29) (Head_Cast_Head :type Integer%20%28by%20ref%29) (Head_Cast_Tail :type Integer%20%28by%20ref%29) (Head :type String%20%28by%20ref%29))
  (return (== Tail_Self_Head Tail_Cast_Head) (== Tail_Self_Tail Tail_Cast_Tail) (== Tail_Self_Head Tail_Cast_Tail) (== Tail_Self_Tail Tail_Cast_Head) (== Head_Self_Head Head_Cast_Head) (== Head_Self_Tail Head_Cast_Tail) (== Head_Self_Head Head_Cast_Tail) (== Head_Self_Tail Head_Cast_Head)))

(fn ComValue
  (params (Self_Head :type Integer%20%28by%20ref%29) (Self_Tail :type Integer%20%28by%20ref%29) (Cast_Head :type Integer%20%28by%20ref%29) (Cast_Tail :type Integer%20%28by%20ref%29) (Function :type String))
  (return (== Self_Head Cast_Head) (== Self_Tail Cast_Tail) (== Self_Head Cast_Tail) (== Self_Tail Cast_Head)))

(fn ReactFunction
  (params (Head%20Equals%20Head :type Boolean%20%28by%20ref%29) (Tails%20Equals%20Tails :type Boolean%20%28by%20ref%29) (Head%20Equals%20Tails :type Boolean%20%28by%20ref%29) (Tails%20Equal%20Heads :type Boolean%20%28by%20ref%29))
  (bind _returnvalue (Utilities|GetDisplayName 0))
  (bind _self self)
  (bind _currentdomino (Variables|Default|GetCurrentDomino))
  (bind _returnvalue_2 (Utilities|GetDisplayName _self))
  (bind _returnvalue_3 (Utilities|GetDisplayName _currentdomino))
  (bind _returnvalue_4 (Utilities|String|Append _returnvalue_2 "_+_" _returnvalue "_+_" _returnvalue_3))
  (Development|PrintString _returnvalue_4 true true "(R=0.019820,G=1.000000,B=0.000000,A=1.000000)" 2e+01)
  (if Tails%20Equals%20Tails
    (Variables|Default|SetIsValid true)
    (Development|PrintString _returnvalue_4 true true "(R=1.000000,G=0.026037,B=0.000000,A=1.000000)" 2e+01)
    (Transformation|SetActorRotation _currentdomino "0,180.000000, 0")
    (bind _asdomino_blueprint (Utilities|Casting|CastToDomino_Blueprint _currentdomino)
      (:then
        (Collision|SetCollisionEnabled (Variables|/Script/Engine.StaticMeshActor|GetStaticMeshComponent _asdomino_blueprint) "NoCollision")
        (Variables|Default|SetPlaced true)
        (Development|PrintString "end of true"))
      (:CastFailed
        (Development|PrintString "suck my ass")))
    (else
      (Variables|Default|SetIsValid false)
      (bind _asdomino_blueprint_2 (Utilities|Casting|CastToDomino_Blueprint _currentdomino))
      (Collision|SetCollisionEnabled (Variables|/Script/Engine.StaticMeshActor|GetStaticMeshComponent _asdomino_blueprint_2) "QueryAndPhysics"))))

(fn NewFunction0
  (params (SelfLocationVector :type Vector%20%28by%20ref%29) (CastLocationVector :type Vector%20%28by%20ref%29) (SelfScale :type Vector%20%28by%20ref%29) (CastScale :type Vector%20%28by%20ref%29))
  (Development|PrintString (Utilities|String|Append (Utilities|String|ToString(Vector) SelfLocationVector) "___" (Utilities|String|ToString(Vector) CastLocationVector)) true true "(R=0.970537,G=0.977903,B=1.000000,A=1.000000)" 5e+01)
  (Development|PrintString (Utilities|String|Append (Utilities|String|ToString(Vector) SelfScale) "___" (Utilities|String|ToString(Vector) CastScale)) true true "(R=1.000000,G=0.000000,B=0.860811,A=1.000000)" 5e+01))

(fn CheckPlayArea
  (return (Math|Geometry|IsPointinBox (Transformation|GetActorLocation) (Variables|Default|GetOrigin) (Variables|Default|GetExtent))))