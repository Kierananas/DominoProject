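; Domino game character that sets up a two-player match on BeginPlay.
; It builds the 28 unique head/tail pairs, spawns a tile actor for each in a value-based grid, then shuffles the tile array.
; It spawns hand-position actors, then deals five tiles per player through a temporary RemovedTiles array, moving them onto those markers.
; Tick only prints a draw reminder when Player 1's hand drops below five.
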(event EventBeginPlay
  (bind _dominotiles (Variables|Default|GetDominoTiles))
  (Utilities|FlowControl|Sequence
    (:then_0
      ;[1 1 1] Feed the set of values from the function into an array, create a loop which for each element in the array spawns, sets the head/tail value of that actor then push into the "Domino Tiles" Array - MK2
      (bind _returnlistofsets (CallFunction|GenerateDominoesPairs))
      (bind _output_get (Variables|Default|SetdominoesPairs _returnlistofsets))
      (bind _result (Utilities|Set|ToArray _output_get))
      (for _array_element _result
        (bind _returnvalue (Game|SpawnActorfromClass "/Game/Blueprints/Domino_Blueprint.Domino_Blueprint_C" (Math|Transform|MakeTransform (+ (+ (* "400.000000, 0, 0" (.head _array_element)) (* "0,400.000000, 0" (.tail _array_element))) "-1100.000000,-1100.000000,-250.000000")) "Undefined" 0 0))
        (Development|PrintString (Utilities|GetDisplayName _returnvalue))
        (Variables|Default|SetDominoBlueprint _returnvalue)
        (Variables|/Game/Blueprints/Domino_Blueprint.Domino_Blueprint_C|Sethead_value _returnvalue (.head _array_element))
        (Variables|/Game/Blueprints/Domino_Blueprint.Domino_Blueprint_C|Settail_value _returnvalue (.tail _array_element))
        (Default|InitData _returnvalue)
        (Utilities|Array|Add _dominotiles _returnvalue))
      (Utilities|Array|Shuffle _dominotiles))
    (:then_1
      (CallFunction|PlayerHandLocations))
    (:then_2
      (CallFunction|PickRandomDominos)
      (bind _output_get_2 (Variables|Default|SetPlayerEnum "NewEnumerator0"))
      (CallFunction|PlaceDominosinHand (Variables|Default|GetPlayer1HandPos) _output_get_2))
    (:then_3
      (CallFunction|PickRandomDominos)
      (bind _output_get_3 (Variables|Default|SetPlayerEnum "NewEnumerator1"))
      (CallFunction|PlaceDominosinHand (Variables|Default|GetPlayer2HandPos) _output_get_3))
    (:then_4
      (Variables|/Game/Blueprints/Domino_Blueprint.Domino_Blueprint_C|SetDominoState (Variables|Default|GetDominoBlueprint) "NewEnumerator0")
      (Variables|/Game/Blueprints/Domino_Blueprint.Domino_Blueprint_C|SetSpawned (Variables|Default|GetDominoBlueprint) true))))

(event Collision|EventActorBeginOverlap
  (params (OtherActor :type Actor%20Object%20Reference)))

(event EventTick
  (params (DeltaSeconds :type Float%20%28single-precision%29))
  (switch Utilities|FlowControl|Switch|SwitchonPlayer_Enum "NewEnumerator0"
    (:NewEnumerator0
      (if (< (Utilities|Array|Length (Variables|Default|GetPlayer1Hand)) 5)
        (Development|PrintString "Player 1 needs to draw card")))))

(fn ConstructionScript)

(fn GenerateDominoesPairs
  (bind _output (LocalVariables|Getoutput))
  (for _index (range 0 6)
    (for _index_2 (range 0 _index)
      (Utilities|Set|Add _output (Utilities|Struct|MakePair _index_2 _index))))
  (return _output))

(fn PickRandomDominos
  (bind _dominotiles (Variables|Default|GetDominoTiles))
  ;[1 1 1] Pick Random Tiles Function - Take a handful of tiles (5) from the set of 28 and place it into another Array
  (for _index (range 0 4)
    (Utilities|Array|Add (Variables|Default|GetRemovedTiles) (Utilities|Array|Get(acopy) _dominotiles))
    (Utilities|Array|RemoveIndex _dominotiles)))

(fn PlayerHandLocations
  ;[1 1 1] Spawn Player 1's Hand Positions (EmptyActor), used to place the dominos in front of the player in a nice order.
  (for _index (range 0 (Variables|Default|GetHand%20Size))
    (bind _returnvalue (Game|SpawnActorfromClass "/Game/Blueprints/player1_1_Blueprint.player1_1_Blueprint_C" (Math|Conversions|ToTransform(Vector) (+ "-1200.000000,-700.000000,10.000000" (* "0.000000,300.000000,30.000000" _index))) "Undefined" 0 0))
    (Utilities|Array|Add (Variables|Default|GetPlayer1HandPos) _returnvalue)
    ;;[1 1 1] Player 2 Hand Positions
    (bind _returnvalue_2 (Game|SpawnActorfromClass "/Game/Blueprints/player2_Blueprint.player2_Blueprint_C" (Math|Conversions|ToTransform(Vector) (+ (* "300.000000,0.000000,30.000000" _index) "-515.000000,1250.000000,10.000000")) "Undefined" 0 0))
    (Utilities|Array|Add (Variables|Default|GetPlayer2HandPos) _returnvalue_2)))

(fn PlaceDominosinHand
  (params (HandPos :type Array%20of%20Actor%20Object%20References) (Player :type Byte))
  (bind _removedtiles (Variables|Default|GetRemovedTiles))
  ;[1 1 1] Moves the randomly selected tiles from the removed array and places them in front of the player.
  (for _index (range 0 (Variables|Default|GetHand%20Size))
    (Transformation|SetActorLocation (Utilities|Array|Get(acopy) _removedtiles _index) (Transformation|GetActorLocation (Utilities|Array|Get(acopy) HandPos _index)) false false))
  (Utilities|FlowControl|Sequence
    (:then_0
      (switch Utilities|FlowControl|Switch|SwitchonPlayer_Enum (Variables|Default|GetPlayerEnum)
        (:NewEnumerator0
          (Variables|Default|SetPlayer1Hand _removedtiles))
        (:NewEnumerator1
          (Variables|Default|SetPlayer2Hand _removedtiles))))
    (:then_1
      (Utilities|Array|Clear _removedtiles))))