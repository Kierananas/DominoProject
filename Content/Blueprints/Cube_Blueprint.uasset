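; Cube_Blueprint is a one-shot placement marker that snaps an overlapping domino into position.
; The first Box overlap passes a DoOnce and moves the overlapping actor, whatever its class, to the cube mesh's world location.
; If that actor is a Domino_Blueprint, it gets its DominoRotation applied, loses mesh collision and stores the move result in Placed, and the cube hides itself.
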(event OnComponentBeginOverlap(Box)
  (params (OverlappedComponent :type Primitive%20Component%20Object%20Reference) (OtherActor :type Actor%20Object%20Reference) (OtherComp :type Primitive%20Component%20Object%20Reference) (OtherBodyIndex :type Integer) (bFromSweep :type Boolean) (SweepResult :type Hit%20Result%20Structure%20%28by%20ref%29))
  (Utilities|FlowControl|DoOnce false
    (:Completed
      (bind _returnvalue (Transformation|SetActorLocation OtherActor (Transformation|GetWorldLocation (Variables|Debug|GetStaticMeshComponent)) false false))
      (bind _asdomino_blueprint (Utilities|Casting|CastToDomino_Blueprint OtherActor))
      (Transformation|SetActorRotation _asdomino_blueprint (Variables|/Game/Blueprints/Domino_Blueprint.Domino_Blueprint_C|GetDomino%20Rotation _asdomino_blueprint))
      (Collision|SetCollisionEnabled (Variables|/Script/Engine.StaticMeshActor|GetStaticMeshComponent _asdomino_blueprint) "NoCollision")
      (Variables|/Game/Blueprints/Domino_Blueprint.Domino_Blueprint_C|SetPlaced _asdomino_blueprint _returnvalue)
      (Rendering|SetActorHiddenInGame true))))

(event EventBeginPlay)

(event EventTick
  (params (DeltaSeconds :type Float%20%28single-precision%29)))

(fn ConstructionScript)